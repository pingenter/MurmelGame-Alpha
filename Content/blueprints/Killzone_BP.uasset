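; Killzone actor that sends the MurmelPlayer_BP player back to a respawn point when an overlap begins.
; After a cast to MurmelPlayer_BP, it teleports the first player actor found to the first RespawnPoint_BP in the level.
; It then zeroes the player mesh's linear and angular physics velocity and plays a 2D spawn sound.
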(event `self.ReceiveActorBeginOverlap`
  (params (OtherActor :type "Actor Object Reference"))
  (bind _outactors (`GameplayStatics.GetAllActorsOfClass` "/Game/blueprints/RespawnPoint_BP.RespawnPoint_BP_C"))
  (bind _asmurmel_player_bp (castclass `/Game/blueprints/MurmelPlayer_BP` "/Game/blueprints/MurmelPlayer_BP.MurmelPlayer_BP_C"))
  (bind _outactors_2 (`GameplayStatics.GetAllActorsOfClass` _asmurmel_player_bp))
  (bind _item (`KismetArrayLibrary.Array_Get` _outactors_2))
  (`self.K2_SetActorLocation` _item (`self.K2_GetActorLocation` (`KismetArrayLibrary.Array_Get` _outactors)) false true)
  (`PrimitiveComponent.SetPhysicsLinearVelocity` (`StaticMeshActor.StaticMeshComponent` _item) (0.0 0.0 0.0) false "None")
  (`PrimitiveComponent.SetPhysicsAngularVelocity` (`StaticMeshActor.StaticMeshComponent` _item) (0.0 0.0 0.0) false "None")
  (`GameplayStatics.PlaySound2D` "/Game/sounds/spawn_Cue.spawn_Cue"))

(fn `UserConstructionScript`)