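; Player Blueprint for a physics-driven ball (Murmel, German for marble), moved by camera-relative forces and viewed through mouse-rotated spring arms.
; A delayed Tick line trace detects airborne state, reducing acceleration in air, and measures horizontal speed to gate input forces at a maximum.
; Looping retriggerable delays damp horizontal velocity while airborne and interpolate velocity toward zero while the handbrake is held.
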(event `self.ReceiveBeginPlay`
  ;[1 1 1] air break
  (`KismetSystemLibrary.RetriggerableDelay` 0.1 :!label _label)
  (if (`self.is in air?`)
    (bind _returnvalue (`PrimitiveComponent.GetPhysicsLinearVelocity` (`self.StaticMeshComponent`) "None"))
    (`PrimitiveComponent.SetPhysicsLinearVelocity` (`self.StaticMeshComponent`) (`KismetMathLibrary.VInterpTo` (`KismetMathLibrary.MakeVector` (.x _returnvalue) (.y _returnvalue) (.z _returnvalue)) (`KismetMathLibrary.MakeVector` 0.0 0.0 (.z _returnvalue)) (`GameplayStatics.GetWorldDeltaSeconds`) 30.0) false "None")
    (goto _label)
    (else
      (goto _label))))

(event `InputAxis|mouse_horizontal`
  (params (AxisValue :type "Float (single-precision)"))
  ;[1 1 1] camera
  (`SceneComponent.K2_AddLocalRotation` (`self.SpringArm1`) (`KismetMathLibrary.MakeRotator` 0.0 0.0 (* (`self.CameraSpeedMultiplier`) AxisValue)) false false))

(event `self.ReceiveTick`
  (params (DeltaSeconds :type "Float (single-precision)"))
  (bind _returnvalue (`SceneComponent.K2_GetComponentLocation` (`self.StaticMeshComponent`)))
  ;[1 1 1] Velocity line trace
  (`KismetSystemLibrary.Delay` 0.1)
  (bind (_outhit _returnvalue_2) (`KismetSystemLibrary.LineTraceSingle` _returnvalue (- _returnvalue (0.0 0.0 150.0)) "TraceTypeQuery1"))
  (bind _output_get (set `self.is in air?` (not _returnvalue_2)))
  (if _output_get
    (set `self.air acceleration` 0.3)
    (else
      (set `self.air acceleration` 1.0)))
  (bind _returnvalue_3 (`PrimitiveComponent.GetPhysicsLinearVelocity` (`self.StaticMeshComponent`) "None"))
  (set `self.CurrentVelocity` (`KismetMathLibrary.VSize` (`KismetMathLibrary.MakeVector` (.x _returnvalue_3) (.y _returnvalue_3)))))

(event `InputAxis|mouse_vertical`
  (params (AxisValue :type "Float (single-precision)"))
  ;[1 1 1] camera
  (`SceneComponent.K2_AddLocalRotation` (`self.SpringArm`) (`KismetMathLibrary.MakeRotator` 0.0 (* (`self.CameraSpeedMultiplier`) AxisValue)) false false))

(event `InputAxis|left_right`
  (params (AxisValue :type "Float (single-precision)"))
  ;[1 1 1] Movement
  (if (<= (`self.CurrentVelocity`) (`self.MaximumVelocity`))
    (bind _returnvalue (* (`self.force_v`) (* (stale `InputAxis|up_down` AxisValue) -1.0)))
    (`PrimitiveComponent.AddForce` (`self.StaticMeshComponent`) (* (* (`KismetMathLibrary.GetDirectionUnitVector` (`SceneComponent.K2_GetComponentLocation` (`self.Camera`)) (`SceneComponent.K2_GetComponentLocation` (`self.StaticMeshComponent`))) (`KismetMathLibrary.MakeVector` _returnvalue _returnvalue)) (`self.air acceleration`)) "None" false)))

(event `InputAxis|up_down`
  (params (AxisValue :type "Float (single-precision)"))
  ;[1 1 1] Movement
  (if (<= (`self.CurrentVelocity`) (`self.MaximumVelocity`))
    (bind _returnvalue (* (* (stale `InputAxis|left_right` AxisValue) 5.0) (`self.force_v`)))
    (`PrimitiveComponent.AddForce` (`self.StaticMeshComponent`) (* (* (`KismetMathLibrary.GreaterGreater_VectorRotator` (`KismetMathLibrary.GetDirectionUnitVector` (`SceneComponent.K2_GetComponentLocation` (`self.Camera`)) (`SceneComponent.K2_GetComponentLocation` (`self.StaticMeshComponent`))) (struct :`Yaw` 90.0)) (`KismetMathLibrary.MakeVector` _returnvalue _returnvalue)) (`self.air acceleration`)) "None" false)))

(event `InputAction|HandBreak`
  (params (Key :type "Key Structure" :default "AnyKey"))
  ;[1 1 1] Bremse
  (:`Pressed`
    (set `self.HandBreakDown` true)
    (`KismetSystemLibrary.RetriggerableDelay` 0.2 :!label _label_2)
    (if (`self.HandBreakDown`)
      (bind _returnvalue (`PrimitiveComponent.GetPhysicsLinearVelocity` (`self.StaticMeshComponent`) "None"))
      (`PrimitiveComponent.SetPhysicsLinearVelocity` (`self.StaticMeshComponent`) (`KismetMathLibrary.VInterpTo` _returnvalue (0.0 0.0 0.0) (`GameplayStatics.GetWorldDeltaSeconds`) (`self.HandBreakReactionTime`)) false "None")
      (goto _label_2)))
  (:`Released`
    (set `self.HandBreakDown` false)))

(fn `UserConstructionScript`)